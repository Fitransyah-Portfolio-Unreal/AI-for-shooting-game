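; Guard NPC character that carries a weapon, takes damage and exposes state, patrol route, team and weapon data, apparently for AI control.
; It spawns its weapon on the hand socket at begin play and forwards fire requests to it.
; State and aiming changes pass to the AnimBP by message, and state sets walk speed.
; Health component events play a hit montage, or ragdoll the mesh once on death.
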(event `self.ReceiveBeginPlay`
  ;[1 1 1] Spawn and attach weapon at begin play
  (bind _returnvalue (`|SpawnActorFromClass` (`self.WeaponClass`) (`/Game/_Blueprints/Shared/BPL_Library.Identity Transform`) "AlwaysSpawn" "OverrideRootScale" self self))
  (bind _output_get (set `self.Weapon` _returnvalue))
  (`self.K2_AttachToComponent` _output_get (`self.Mesh`) "WeaponSocket" "SnapToTarget" "SnapToTarget" "SnapToTarget" true))

(event `self.HealthComponent.OnDamageTaken`
  ;[1 1 1] On taking damage action
  (`self.PlayAnimMontage` "/Game/Animation/Hit_Montage.Hit_Montage"))

(event `self.HealthComponent.OnDeath`
  (bind _mesh (`self.Mesh`))
  ;[1 1 1] On Death action
  (`/Engine/EditorBlueprintResources/StandardMacros.DoOnce` false
    (:`Completed`
      (`PrimitiveComponent.SetCollisionProfileName` _mesh "Ragdoll" true)
      (`SkeletalMeshComponent.SetAllBodiesSimulatePhysics` _mesh true)
      (`PrimitiveComponent.WakeAllRigidBodies` _mesh)
      (`PrimitiveComponent.SetCollisionEnabled` (`self.CapsuleComponent`) "NoCollision")
      (`KismetSystemLibrary.PrintString` (`KismetStringLibrary.Concat_StrStr` (`KismetSystemLibrary.GetDisplayName` self) " Died!")))))

(event `/Game/_Blueprints/Shared/BPI_AI_Helper.NotifyStateChanged`
  (params (`New State` :type "/Game/_AI/NPC_States Enum" :default "NewEnumerator0"))
  ;[1 1 1] On State Changed
  (message `/Game/_Blueprints/Shared/BPI_AI_Helper.NotifyStateChanged` (`SkeletalMeshComponent.GetAnimInstance` (`self.Mesh`)) `New State`))

(event `/Game/_Blueprints/Shared/BPI_AI_Helper.ModifyMovementSpeed`
  (params (State :type "/Game/_AI/NPC_States Enum" :default "NewEnumerator0"))
  ;[1 1 1] Update character movement by current state
  (set `CharacterMovementComponent.MaxWalkSpeed` (select `/Game/_AI/NPC_States` State :`NewEnumerator0` 160.0 :`NewEnumerator1` 160.0 :`NewEnumerator2` 400.0 :`NewEnumerator3` 600.0 :!type "Float (single-precision)") (`self.CharacterMovement`)))

(event `/Game/_Blueprints/Shared/BPI_AI_Helper.ModifyAimingStance`
  (params (IsAiming :type Boolean))
  ;[1 1 1] Updating aiming boolean in AnimBP
  (message `/Game/_Blueprints/Shared/BPI_AI_Helper.ModifyAimingStance` (`SkeletalMeshComponent.GetAnimInstance` (`self.Mesh`)) IsAiming))

(event `/Game/_Blueprints/Shared/BPI_AI_Helper.TryShotEquippedWeapon`
  ;[1 1 1] Try shoot gun via interface
  (bind _weapon (`self.Weapon`)
    (:`then`
      (`/Game/_Blueprints/Weapons/WeaponBase.OnFireRequested` _weapon))
    (:`else`)))

(fn `GetIsDead`
  (returns (Dead :type Boolean))
  (return (`/Game/_Blueprints/Shared/HealthComponent.IsDead` (`self.HealthComponent`))))

(fn `GetPatrolRoute`
  (returns (PatrolRoute :type "/Game/_Blueprints/NPC/PatrolRouteSystem Object Reference"))
  (return (`self.MyPatrolPath`)))

(fn `GetTeamID`
  (returns (IsPlayer :type Boolean))
  (return false))

(fn `GetWeapon`
  (returns (HasWeapon :type Boolean) (Weapon :type "/Game/_Blueprints/Weapons/WeaponBase Object Reference"))
  (bind _weapon (`self.Weapon`))
  (return (`KismetSystemLibrary.IsValid` _weapon) _weapon))

(fn `GetWeaponRange`
  (returns (Range :type "Float (double-precision)"))
  (return (`/Game/_Blueprints/Weapons/WeaponBase.Weapon Range` (`self.Weapon`))))

(fn `UserConstructionScript`)